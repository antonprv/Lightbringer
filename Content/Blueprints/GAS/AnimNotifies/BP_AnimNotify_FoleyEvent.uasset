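; Anim notify that triggers foley sounds, chosen by a gameplay tag event, from animations.
; Unless the animation is blending out, it passes the event, side, volume and pitch to the owner's AC_FoleyEvents component.
; Without that component, it plays the matching DefaultBank sound in 2D.
; The notify's displayed name uses the last segment of the event tag.
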(fn `GetNotifyName`
  (returns (ReturnValue :type String))
  (return (`KismetTextLibrary.Conv_TextToString` (`|FormatText` "FoleyEvent: {Type}" (`.RightS` (`KismetStringLibrary.Split` (`BlueprintGameplayTagLibrary.GetDebugStringFromGameplayTag` (`self.Event`)) "." "IgnoreCase" "FromEnd"))))))

(fn `Received_Notify`
  (params (MeshComp :type "SkeletalMeshComponent Object Reference") (Animation :type "AnimSequenceBase Object Reference") (EventReference :type "AnimNotifyEventReference Structure (by ref)"))
  (returns (ReturnValue :type Boolean))
  (locals (FoleyEventComponent :type "/Game/Assets/External/GAS/Audio/Foley/AC_FoleyEvents Object Reference"))
  (bind _returnvalue (`Actor.GetComponentByClass` (`ActorComponent.GetOwner` (`local.MeshComp`)) "/Game/Assets/External/GAS/Audio/Foley/AC_FoleyEvents.AC_FoleyEvents_C"))
  (if (not (`AnimNotifyLibrary.IsBlendingOut` EventReference))
    (`/Engine/EditorBlueprintResources/StandardMacros.IsValid` _returnvalue
      (:`Is Valid`
        (`/Game/Assets/External/GAS/Audio/Foley/AC_FoleyEvents.PlayFoleyEvent` _returnvalue (`self.Event`) (make `/Game/Assets/External/GAS/Audio/Foley/S_FoleyEventParams` (`self.Side`) (`self.VolumeMultiplier`) (`self.PitchMultiplier`)))
        (return true))
      (:`Is Not Valid`
        (`GameplayStatics.PlaySound2D` (`/Game/Assets/External/GAS/Audio/Foley/DABP_FoleyAudioBank.GetSoundFromFoleyEvent` (`self.DefaultBank`) (`self.Event`)) (`self.VolumeMultiplier`) (`self.PitchMultiplier`) 0.0 null null)))))